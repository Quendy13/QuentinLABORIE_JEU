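; BP_PuzzleGate is a horror template gate that opens once enough puzzle items have been collected.
; CollectItem increments a counter and, when it reaches the configured maximum, calls OpenDoor a single time through a DoOnce.
; OpenDoor plays a timeline that lerps the Door component's yaw to swing it open.
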(event `self.ReceiveBeginPlay`)

(event `OpenDoor`
  (bind (_direction _door_rot) (`Timeline|Door_TL`)
    (:`Update`
      (`SceneComponent.K2_SetRelativeRotation` (`self.Door`) (`KismetMathLibrary.MakeRotator` 0.0 0.0 (`KismetMathLibrary.Lerp` 0.0 120.0 _door_rot)) false false))))

(event `CollectItem`
  (`/Engine/EditorBlueprintResources/StandardMacros.IncrementInt` (`self.CurrentItemsCollected?`)
    (:`  `
      (if (>= (`self.CurrentItemsCollected?`) (`self.MaxItemsCollectable`))
        (`/Engine/EditorBlueprintResources/StandardMacros.DoOnce` false
          (:`Completed`
            (`self.OpenDoor`)))))))

(fn `UserConstructionScript`)