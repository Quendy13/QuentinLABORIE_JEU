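; BP_Box is a hiding spot that the horror character enters and leaves through interaction.
; Its Interaction event casts player 0 to BP_HorrorCharacter and uses a FlipFlop to alternate between the two states.
; Entering teleports the capsule to the static mesh and sets IsHidden.
; Leaving teleports it to the Box component's XY at a hardcoded world height and clears the flag.
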(event `/Game/HorrorTemplate/Blueprint/Interfaces/BPI_Interaction.Interaction`
  (bind (_returnvalue_x _returnvalue_y) (`KismetMathLibrary.BreakVector` (`SceneComponent.K2_GetComponentLocation` (`self.Box`))))
  (bind _asbp_horror_character (cast `/Game/HorrorTemplate/Blueprint/Character/BP_HorrorCharacter` (`GameplayStatics.GetPlayerCharacter` 0))
    (:`then`
      (`/Engine/EditorBlueprintResources/StandardMacros.FlipFlop`
        (:`A`
          (`SceneComponent.K2_SetWorldTransform` (`Character.CapsuleComponent` _asbp_horror_character) (`KismetMathLibrary.MakeTransform` (`SceneComponent.K2_GetComponentLocation` (`self.StaticMesh`))) false true)
          (set `/Game/HorrorTemplate/Blueprint/Character/BP_HorrorCharacter.bIsHidden` true _asbp_horror_character))
        (:`B`
          (`SceneComponent.K2_SetWorldTransform` (`Character.CapsuleComponent` _asbp_horror_character) (`KismetMathLibrary.MakeTransform` (`KismetMathLibrary.MakeVector` _returnvalue_x _returnvalue_y 50.0)) false true)
          (set `/Game/HorrorTemplate/Blueprint/Character/BP_HorrorCharacter.bIsHidden` false _asbp_horror_character))))
    (:`CastFailed`
      (`KismetSystemLibrary.PrintString` "Erreur de cast"))))

(fn `UserConstructionScript`)